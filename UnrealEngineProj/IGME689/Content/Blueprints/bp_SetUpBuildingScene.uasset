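; Level setup actor that prepares an ArcGIS building scene for what appears to be a puzzle game.
; On BeginPlay it stores a random numeric solution string, finds the ArcGIS map actor and caches its first layer as the building scene layer.
; It then moves the map origin to a hard-coded WGS84 building location, calls a still-empty LoadPuzzles event and spawns the first-person player after a fixed delay.
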(event Custom|GetSceneLayer
  ;[0.15 0.15 0.15 0.5] Gets building scene layer
  (bind _returnvalue (Actor|GetActorOfClass "/Script/ArcGISMapsSDK.ArcGISMapActor"))
  (bind _output_get (Variables|Default|SetMapComponent _returnvalue))
  (bind _returnvalue_2 (Class|ArcGISMapComponent|GetMap (Variables|/Script/ArcGISMapsSDK.ArcGISMapActor|GetMapComponent _output_get)))
  (bind _returnvalue_3 (Class|ArcGISMap|GetLayers _returnvalue_2))
  (bind _returnvalue_4 (Class|ArcGISLayerCollection|GetSize _returnvalue_3))
  (if (!= _returnvalue_4 0)
    (bind _output_get_2 (Variables|Default|SetBuildingSceneLayer (Class|ArcGISLayerCollection|At _returnvalue_3)))
    (bind _returnvalue_5 (Class|ArcGISLayer|GetName _output_get_2))
    (Development|PrintString _returnvalue_5)))

(event Custom|LoadPuzzles)

(event EventBeginPlay
  ;[0.15 0.15 0.15 0.5] Setting solution
  (Variables|Default|SetSolution (Utilities|String|ToString(Integer) (Math|Random|RandomInteger 10000)))
  (CallFunction|GetSceneLayer)
  ;[0.15 0.15 0.15 0.5] Setting map location
  (bind _output_get (Variables|Default|SetBuildingLocation "172.637113,-43.529995,7.000000"))
  (bind _returnvalue (Class|ArcGISSpatialReference|WGS84))
  (bind _returnvalue_2 (Class|ArcGISPoint|CreateArcGISPointwithXYZSpatialReference (.x _output_get) (.y _output_get) (.z _output_get) _returnvalue))
  (Class|ArcGISMapComponent|SetOriginPosition (Variables|/Script/ArcGISMapsSDK.ArcGISMapActor|GetMapComponent (Variables|Default|GetMapComponent)) _returnvalue_2)
  (CallFunction|LoadPuzzles)
  (Utilities|FlowControl|Delay 5.0)
  (bind _returnvalue_3 (Game|SpawnActorfromClass "/Game/FirstPerson/Blueprints/BP_FirstPersonCharacter.BP_FirstPersonCharacter_C" (Math|Transform|MakeTransform "0, 0, 0" "0, 0, 0" "1.000000,1.000000,1.000000") "Undefined" "MultiplyWithRoot" 0 0))
  (Variables|Default|SetPlayer _returnvalue_3))

(event Collision|EventActorBeginOverlap
  (params (OtherActor :type Actor%20Object%20Reference)))

(event EventTick
  (params (DeltaSeconds :type Float%20%28single-precision%29)))

(fn ConstructionScript)