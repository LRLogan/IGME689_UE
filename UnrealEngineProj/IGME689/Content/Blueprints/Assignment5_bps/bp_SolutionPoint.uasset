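; A collectible key fragment that the first-person player picks up with the E key while standing near it.
; Overlapping its box enables input and shows a text prompt, and leaving disables both.
; Pressing E registers the point once with the Bp_SetUpBuildingScene actor, hides itself and updates the HUD progress counter.
; When the collected count reaches the required number, the HUD widget reveals the code.
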(event OnComponentBeginOverlap(Box)
  (params (OverlappedComponent :type Primitive%20Component%20Object%20Reference) (OtherActor :type Actor%20Object%20Reference) (OtherComp :type Primitive%20Component%20Object%20Reference) (OtherBodyIndex :type Integer) (bFromSweep :type Boolean) (SweepResult :type Hit%20Result%20Structure%20%28by%20ref%29))
  (Utilities|Casting|CastToBP_FirstPersonCharacter OtherActor)
  (Input|EnableInput (Game|GetPlayerController 0))
  (Rendering|SetVisibility (Variables|Default|GetTextRender) true false))

(event EventBeginPlay)

(event Collision|EventActorEndOverlap
  (params (OtherActor :type Actor%20Object%20Reference))
  (Utilities|Casting|CastToBP_FirstPersonCharacter OtherActor)
  (Input|DisableInput (Game|GetPlayerController 0))
  (Rendering|SetVisibility (Variables|Default|GetTextRender) false false))

(event Input|KeyboardEvents|E
  (params (Key :type Key%20Structure :default "None"))
  ;[0.15 0.15 0.15 0.5] Player clicked on object
  (:Pressed
    (bind _returnvalue (Actor|GetActorOfClass "/Game/Blueprints/Assignment5_bps/bp_SetUpBuildingScene.bp_SetUpBuildingScene_C"))
    (Variables|Default|SetMainSceneBP _returnvalue)
    (if (not (Utilities|Array|ContainsItem (Variables|/Game/Blueprints/Assignment5_bps/bp_SetUpBuildingScene.bp_SetUpBuildingScene_C|GetPointsClickedOn (Variables|Default|GetMainSceneBP)) self))
      (Utilities|Array|Add (Variables|/Game/Blueprints/Assignment5_bps/bp_SetUpBuildingScene.bp_SetUpBuildingScene_C|GetPointsClickedOn (Variables|Default|GetMainSceneBP)) self)
      (Rendering|SetVisibility (Variables|Default|GetDefaultSceneRoot) false true)
      (Variables|/Game/Blueprints/Assignment5_bps/bp_SetUpBuildingScene.bp_SetUpBuildingScene_C|SetCurNumPoints (Variables|Default|GetMainSceneBP) (+ (Variables|/Game/Blueprints/Assignment5_bps/bp_SetUpBuildingScene.bp_SetUpBuildingScene_C|GetCurNumPoints (Variables|Default|GetMainSceneBP)) 1))
      (Rendering|Components|TextRender|SetText (Variables|/Game/Blueprints/Assignment5_bps/wbp_EscapeRoomHUD.wbp_EscapeRoomHUD_C|GetCollectionProgressText (Variables|/Game/Blueprints/Assignment5_bps/bp_SetUpBuildingScene.bp_SetUpBuildingScene_C|GetHUDWidget (Variables|Default|GetMainSceneBP))) (Utilities|Text|ToText(String) (Utilities|String|Append "Collect key fragments: " (Utilities|String|ToString(Integer) (Variables|/Game/Blueprints/Assignment5_bps/bp_SetUpBuildingScene.bp_SetUpBuildingScene_C|GetCurNumPoints (Variables|Default|GetMainSceneBP))) " / " (Utilities|String|ToString(Integer) (Variables|/Game/Blueprints/Assignment5_bps/bp_SetUpBuildingScene.bp_SetUpBuildingScene_C|GetNumPointsNeeded (Variables|Default|GetMainSceneBP))))))
      ;[0.15 0.15 0.15 0.5] Check for compleation
      (if (>= (Variables|/Game/Blueprints/Assignment5_bps/bp_SetUpBuildingScene.bp_SetUpBuildingScene_C|GetCurNumPoints (Variables|Default|GetMainSceneBP)) (Variables|/Game/Blueprints/Assignment5_bps/bp_SetUpBuildingScene.bp_SetUpBuildingScene_C|GetNumPointsNeeded (Variables|Default|GetMainSceneBP)))
        (Default|ShowCode (Variables|/Game/Blueprints/Assignment5_bps/bp_SetUpBuildingScene.bp_SetUpBuildingScene_C|GetHUDWidget (Variables|Default|GetMainSceneBP)))))))

(fn ConstructionScript)