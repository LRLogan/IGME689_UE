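; Scene setup actor for a building escape-room level built on an ArcGIS map.
; On BeginPlay it rolls a random numeric solution, grabs the map's first layer and sets the map origin to a fixed WGS84 location.
; It hides all Bp_SolutionPoint actors, then randomly reveals a required number of distinct ones, redrawing on duplicates.
; After a five-second delay it spawns the first-person character and adds the escape-room HUD.
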(event Custom|CreateUI
  (bind _returnvalue (UserInterface|CreateWidget "/Game/Blueprints/Assignment5_bps/wbp_EscapeRoomHUD.wbp_EscapeRoomHUD_C" (Game|GetPlayerController 0)))
  (bind _output_get (Variables|Default|SetHUDWidget _returnvalue))
  (UserInterface|Viewport|AddtoViewport _output_get 0))

(event Custom|LoadPuzzles
  (bind _curpuzzlepoint (Variables|Default|GetCurPuzzlePoint))
  (bind _returnvalue (Utilities|GetObjectName _curpuzzlepoint))
  ;[0.15 0.15 0.15 0.5] Gets the location of all the puzzle points set in the world
  (bind _outactors (Actor|GetAllActorsOfClass "/Game/Blueprints/Assignment5_bps/bp_SolutionPoint.bp_SolutionPoint_C"))
  (bind _output_get (Variables|Default|SetPosssibleSolPointLocations _outactors))
  (for _array_element _output_get
    (Rendering|SetVisibility (Variables|/Script/Engine.Actor|GetRootComponent _array_element) false true))
  ;[0.15 0.15 0.15 0.5] Getting / Setting puzzle item locations
  (for _index (range 0 (- (Variables|Default|GetNumPointsNeeded) 1))
    (CallFunction|CheckGetLocation)
    (Utilities|Map|Add (Variables|Default|GetFinalSolPointLocations) _returnvalue _curpuzzlepoint)
    (Rendering|SetVisibility (Variables|/Script/Engine.Actor|GetRootComponent _curpuzzlepoint) true true)
    (Development|PrintString _returnvalue)))

(event Custom|CheckGetLocation
  ;[0.15 0.15 0.15 0.5] Ensures the location gottes is not already in use
  (bind _output_get (Variables|Default|SetContainsPoint true))
  (while _output_get
    (bind _newparam (CallFunction|GetLocation))
    (Variables|Default|SetCurPuzzlePoint _newparam)
    (Variables|Default|SetContainsPoint (Utilities|Map|Contains (Variables|Default|GetFinalSolPointLocations) (Utilities|GetObjectName _newparam)))))

(event Custom|GetSceneLayer
  ;[0.15 0.15 0.15 0.5] Gets building scene layer
  (bind _returnvalue (Actor|GetActorOfClass "/Script/ArcGISMapsSDK.ArcGISMapActor"))
  (bind _output_get (Variables|Default|SetMapComponent _returnvalue))
  (bind _returnvalue_2 (Class|ArcGISMapComponent|GetMap (Variables|/Script/ArcGISMapsSDK.ArcGISMapActor|GetMapComponent _output_get)))
  (bind _returnvalue_3 (Class|ArcGISMap|GetLayers _returnvalue_2))
  (bind _returnvalue_4 (Class|ArcGISLayerCollection|GetSize _returnvalue_3))
  (if (!= _returnvalue_4 0)
    (bind _output_get_2 (Variables|Default|SetBuildingSceneLayer (Class|ArcGISLayerCollection|At _returnvalue_3)))
    (bind _returnvalue_5 (Class|ArcGISLayer|GetName _output_get_2))
    (Development|PrintString _returnvalue_5)))

(event EventBeginPlay
  (Input|SetInputModeGameOnly (Game|GetPlayerController 0) false)
  ;[0.15 0.15 0.15 0.5] Setting solution
  (Variables|Default|SetSolution (Utilities|String|ToString(Integer) (Math|Random|RandomInteger 10000)))
  (CallFunction|GetSceneLayer)
  ;[0.15 0.15 0.15 0.5] Setting map location
  (bind _output_get (Variables|Default|SetBuildingLocation "172.637113,-43.529995,7.000000"))
  (bind _returnvalue (Class|ArcGISSpatialReference|WGS84))
  (bind _returnvalue_2 (Class|ArcGISPoint|CreateArcGISPointwithXYZSpatialReference (.x _output_get) (.y _output_get) (.z _output_get) _returnvalue))
  (Class|ArcGISMapComponent|SetOriginPosition (Variables|/Script/ArcGISMapsSDK.ArcGISMapActor|GetMapComponent (Variables|Default|GetMapComponent)) _returnvalue_2)
  (CallFunction|LoadPuzzles)
  (Utilities|FlowControl|Delay 5.0)
  (bind _returnvalue_3 (Game|SpawnActorfromClass "/Game/FirstPerson/Blueprints/BP_FirstPersonCharacter.BP_FirstPersonCharacter_C" (Math|Transform|MakeTransform "0, 0, 0" "0, 0, 0" "1.000000,1.000000,1.000000") "Undefined" "MultiplyWithRoot" 0 0))
  (Variables|Default|SetPlayer _returnvalue_3)
  (CallFunction|CreateUI))

(event Collision|EventActorBeginOverlap
  (params (OtherActor :type Actor%20Object%20Reference)))

(event EventTick
  (params (DeltaSeconds :type Float%20%28single-precision%29)))

(fn ConstructionScript)

(fn GetLocation
  (bind _posssiblesolpointlocations (Variables|Default|GetPosssibleSolPointLocations))
  (if (Utilities|Array|IsNotEmpty _posssiblesolpointlocations)
    (return (Utilities|Array|Get(acopy) _posssiblesolpointlocations (Math|Random|RandomInteger (Utilities|Array|Length _posssiblesolpointlocations))))
    (else
      (Development|PrintText "EMPTY ARRAY"))))