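; A keypad-locked door that ends the game with a win when opened.
; On setup it creates a hidden Wbp_numpad widget and, after a short delay, copies the solution from Bp_SetUpBuildingScene into it.
; While the player overlaps it, prompt texts show and E toggles the numpad and mouse input; leaving hides it again.
; OpenDoor flags game over on the scene Blueprint and shows its HUD win screen.
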(event OnComponentBeginOverlap(Box)
  (params (OverlappedComponent :type Primitive%20Component%20Object%20Reference) (OtherActor :type Actor%20Object%20Reference) (OtherComp :type Primitive%20Component%20Object%20Reference) (OtherBodyIndex :type Integer) (bFromSweep :type Boolean) (SweepResult :type Hit%20Result%20Structure%20%28by%20ref%29))
  (Utilities|Casting|CastToBP_FirstPersonCharacter OtherActor)
  (Input|EnableInput (Game|GetPlayerController 0))
  (Rendering|SetVisibility (Variables|Default|GetTextRender) true false))

(event Custom|OpenDoor
  ;[0.15 0.15 0.15 0.5] Player win
  (Development|PrintText "Opened door!")
  (bind _returnvalue (Actor|GetActorOfClass "/Game/Blueprints/Assignment5_bps/bp_SetUpBuildingScene.bp_SetUpBuildingScene_C"))
  (bind _output_get (Variables|Default|SetMainSceneBP _returnvalue))
  (Variables|/Game/Blueprints/Assignment5_bps/bp_SetUpBuildingScene.bp_SetUpBuildingScene_C|SetIsGameOver _output_get true)
  (bind _output_get_2 (Variables|Default|SetHUDWidget (Variables|/Game/Blueprints/Assignment5_bps/bp_SetUpBuildingScene.bp_SetUpBuildingScene_C|GetHUDWidget (Variables|Default|GetMainSceneBP))))
  (Default|ShowDefaultEndState _output_get_2)
  (Widget|SetVisibility (Variables|/Game/Blueprints/Assignment5_bps/wbp_EscapeRoomHUD.wbp_EscapeRoomHUD_C|GetWinText _output_get_2) "Visible"))

(event Custom|SetupDoor
  ;[0.15 0.15 0.15 0.5] Used when the game is reset due to BeginPlay not bein called
  (bind _returnvalue (UserInterface|CreateWidget "/Game/Blueprints/Assignment5_bps/wbp_numpad.wbp_numpad_C"))
  (Widget|SetVisibility _returnvalue "Hidden")
  (bind _output_get (Variables|Default|SetNumpad _returnvalue))
  (UserInterface|Viewport|AddtoViewport _output_get 0)
  ;[0.15 0.15 0.15 0.5] Set door Solution
  (bind _returnvalue_2 (Actor|GetActorOfClass "/Game/Blueprints/Assignment5_bps/bp_SetUpBuildingScene.bp_SetUpBuildingScene_C"))
  (Utilities|FlowControl|Delay 0.2)
  (bind _output_get_2 (Variables|/Game/Blueprints/Assignment5_bps/wbp_numpad.wbp_numpad_C|SetDoorSolution _output_get (Variables|/Game/Blueprints/Assignment5_bps/bp_SetUpBuildingScene.bp_SetUpBuildingScene_C|GetSolution _returnvalue_2)))
  (Development|PrintString _output_get_2))

(event EventBeginPlay
  (CallFunction|SetupDoor))

(event Collision|EventActorEndOverlap
  (params (OtherActor :type Actor%20Object%20Reference))
  (bind _returnvalue (Game|GetPlayerController 0))
  (Utilities|Casting|CastToBP_FirstPersonCharacter OtherActor)
  (Input|DisableInput (Game|GetPlayerController 0))
  (Rendering|SetVisibility (Variables|Default|GetTextRender) false false)
  (Widget|SetVisibility (Variables|Default|GetNumpad) "Hidden")
  (Input|SetInputModeGameOnly _returnvalue false)
  (Variables|/Script/Engine.PlayerController|SetbShowMouseCursor _returnvalue false))

(event Input|KeyboardEvents|E
  (params (Key :type Key%20Structure :default "None"))
  (bind _returnvalue (Game|GetPlayerController 0))
  (bind _numpad (Variables|Default|GetNumpad))
  ;[0.15 0.15 0.15 0.5] When clicking on door
  (:Pressed
    (Utilities|FlowControl|FlipFlop
      (:A
        (Widget|SetVisibility _numpad "Visible")
        (Input|SetInputModeGameandUI _returnvalue _numpad "DoNotLock" true false)
        (Variables|/Script/Engine.PlayerController|SetbShowMouseCursor _returnvalue true))
      (:B
        (Widget|SetVisibility _numpad "Hidden")
        (Input|SetInputModeGameOnly _returnvalue false)
        (Variables|/Script/Engine.PlayerController|SetbShowMouseCursor _returnvalue false)))))

(fn ConstructionScript)