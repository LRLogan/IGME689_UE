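; bp_SolutionPoint is an interactable actor that the player can hide by pressing E while nearby.
; A BP_FirstPersonCharacter overlapping its Box enables the actor's input and shows a TextRender, and ending overlap with the actor reverses both.
; Pressing E hides the root component and its children without destroying the actor or changing collision.
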(event OnComponentBeginOverlap(Box)
  (params (OverlappedComponent :type Primitive%20Component%20Object%20Reference) (OtherActor :type Actor%20Object%20Reference) (OtherComp :type Primitive%20Component%20Object%20Reference) (OtherBodyIndex :type Integer) (bFromSweep :type Boolean) (SweepResult :type Hit%20Result%20Structure%20%28by%20ref%29))
  (Utilities|Casting|CastToBP_FirstPersonCharacter OtherActor)
  (Input|EnableInput (Game|GetPlayerController 0))
  (Rendering|SetVisibility (Variables|Default|GetTextRender) true false))

(event EventBeginPlay)

(event Collision|EventActorEndOverlap
  (params (OtherActor :type Actor%20Object%20Reference))
  (Utilities|Casting|CastToBP_FirstPersonCharacter OtherActor)
  (Input|DisableInput (Game|GetPlayerController 0))
  (Rendering|SetVisibility (Variables|Default|GetTextRender) false false))

(event Input|KeyboardEvents|E
  (params (Key :type Key%20Structure :default "None"))
  (:Pressed
    (Rendering|SetVisibility (Variables|Default|GetDefaultSceneRoot) false true)))

(fn ConstructionScript)