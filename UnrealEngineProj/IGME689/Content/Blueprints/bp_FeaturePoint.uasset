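; Feature point actor for an ArcGIS map that places itself at a WGS84 longitude and latitude.
; BeginPlay caches the map actor and ArcGIS pawn, and SpawnFeaturePoints positions the actor's location component, set to sit on the ground.
; UpdatePos moves the pawn to given coordinates at a fixed altitude, recenters the map origin there and prints the result.
; Tick checks whether the view has finished drawing but does nothing with it yet.
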(event EventBeginPlay
  (bind _returnvalue (Actor|GetActorOfClass "/Script/ArcGISMapsSDK.ArcGISMapActor"))
  (Variables|Default|SetMapComponent _returnvalue)
  (bind _returnvalue_2 (Actor|GetActorOfClass "/Script/ArcGISSamples.ArcGISPawn"))
  (Variables|Default|SetPawn _returnvalue_2))

(event Collision|EventActorBeginOverlap
  (params (OtherActor :type Actor%20Object%20Reference)))

(event EventTick
  (params (DeltaSeconds :type Float%20%28single-precision%29))
  (bind _returnvalue (Class|ArcGISMapComponent|GetView (Class|ArcGISMapComponent|GetMapComponent (Variables|Default|GetMapComponent))))
  (bind _returnvalue_2 (Class|ArcGISView|GetDrawStatus _returnvalue))
  ;[0.15 0.15 0.15 0.5] Can connect car to this / this ensures that everything is loaded
  (if (Utilities|Enum|Equal(Enum) _returnvalue_2 "Completed")
    _))

(fn ConstructionScript)

(fn UpdatePos
  (params (Long :type Float%20%28double-precision%29) (Lat :type Float%20%28double-precision%29))
  (bind _mapcomponent (Variables|Default|GetMapComponent))
  (bind _mapcomponent_2 (Variables|/Script/ArcGISMapsSDK.ArcGISMapActor|GetMapComponent _mapcomponent))
  (bind _returnvalue (Class|ArcGISMapComponent|GetOriginPosition _mapcomponent_2))
  (bind _returnvalue_2 (Class|ArcGISSpatialReference|WGS84))
  (bind _returnvalue_3 (Class|ArcGISPoint|CreateArcGISPointwithXYZSpatialReference Long Lat 1.4e+03 _returnvalue_2))
  (Class|ArcGISLocationComponent|SetPosition (Actor|GetComponentbyClass (Variables|Default|GetPawn) "/Script/ArcGISMapsSDK.ArcGISLocationComponent") _returnvalue_3)
  (bind _returnvalue_4 (Class|ArcGISPoint|CreateArcGISPointwithXYZSpatialReference Long Lat 0.0 _returnvalue_2))
  (Class|ArcGISMapComponent|SetOriginPosition _mapcomponent_2 _returnvalue_4)
  (bind _returnvalue_5 (Class|ArcGISPoint|GetX _returnvalue))
  (bind _returnvalue_6 (Class|ArcGISPoint|GetY _returnvalue))
  (Development|PrintString (Utilities|String|Append "Long " (Utilities|String|ToString(Float) _returnvalue_5) "Lat " (Utilities|String|ToString(Float) _returnvalue_6) "Called from UpdatePos")))

(fn SpawnFeaturePoints
  (params (Long :type Float%20%28double-precision%29) (Lat :type Float%20%28double-precision%29))
  (bind _arcgislocation (Variables|Default|GetArcGISLocation))
  (bind _returnvalue (Class|ArcGISSpatialReference|WGS84))
  (bind _returnvalue_2 (Class|ArcGISPoint|CreateArcGISPointwithXYZSpatialReference Long Lat 0.0 _returnvalue))
  (Class|ArcGISLocationComponent|SetPosition _arcgislocation _returnvalue_2)
  (Class|ArcGISLocationComponent|SetSurfacePlacementMode _arcgislocation "OnTheGround"))